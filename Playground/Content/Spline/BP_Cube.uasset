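; BP_Cube is an actor that travels along a spline path when play begins.
; On BeginPlay it finds a BP_SplinePath in the level and starts a timeline, with play rate set from TimeToCompleteInSec.
; Each update maps the timeline track to a distance along the spline's length and sets the actor's world location and rotation from that point.
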(event `self.ReceiveBeginPlay`
  (bind _returnvalue (`GameplayStatics.GetActorOfClass` "/Game/Spline/BP_SplinePath.BP_SplinePath_C"))
  (set `self.SplineREF` _returnvalue)
  (`self.MoveObject`))

(event `MoveObject`
  (bind _spline (`/Game/Spline/BP_SplinePath.Spline` (`self.SplineREF`)))
  (`TimelineComponent.SetPlayRate` (`self.MoveObjectT`) (/ 1.0 (`self.TimeToComplete(inSec)`)))
  (bind (_direction _movetrack) (`Timeline|MoveObjectT`)
    (:`Update`
      (bind _returnvalue (`KismetMathLibrary.Lerp` 0.0 (`SplineComponent.GetSplineLength` (`/Game/Spline/BP_SplinePath.Spline` (`self.SplineREF`))) _movetrack))
      (`self.K2_SetActorTransform` (`KismetMathLibrary.MakeTransform` (`SplineComponent.GetLocationAtDistanceAlongSpline` _spline _returnvalue "World") (`SplineComponent.GetRotationAtDistanceAlongSpline` _spline _returnvalue "World"))))))

(fn `UserConstructionScript`)